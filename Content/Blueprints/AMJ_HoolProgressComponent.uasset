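; AMJ_HoolProgressComponent tracks how many computers exist and how many are destroyed, and ends the game when all are down.
; Spawn calls raise the total, destroy calls raise the destroyed count and respawn calls lower it.
; When the destroyed count equals the total, it casts the game mode to AMJ-GameModeBase and calls GameOver with false.
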(fn `OnComputerDestroy`
  (`/Engine/EditorBlueprintResources/StandardMacros.IncrementInt` (`self.NumOfDestroyedComputers`)
    (:`  `
      (if (== (`self.NumOfDestroyedComputers`) (`self.NumOfComputers`))
        (bind _asamj_game_mode_base (cast `/Game/Blueprints/AMJ-GameModeBase` (`GameplayStatics.GetGameMode`)))
        (`/Game/Blueprints/AMJ-GameModeBase.GameOver` _asamj_game_mode_base false)))))

(fn `OnComputerRespawn`
  (`/Engine/EditorBlueprintResources/StandardMacros.DecrementInt` (`self.NumOfDestroyedComputers`)))

(fn `OnSpawnedComputer`
  (`/Engine/EditorBlueprintResources/StandardMacros.IncrementInt` (`self.NumOfComputers`)))