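; Destructible desk workstation that lets AMJ-Programmer actors code while they overlap its box trigger.
; Damage lowers health on an HP bar widget; at zero it notifies programmers, hides itself, disables collision, and triggers camera shake, a bam effect and a spawned destructible stand-in.
; A Tick countdown then restores visibility, collision and full health.
; Spawn, destruction and respawn are reported to the game mode's progress component.
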(event `self.ReceiveBeginPlay`
  (set `self.Health` (`self.MaxHealth`))
  (`self.SetHealthBar`)
  (bind _asamj_game_mode_base (cast `/Game/Blueprints/AMJ-GameModeBase` (`GameplayStatics.GetGameMode`)))
  (`/Game/Blueprints/AMJ_HoolProgressComponent.OnSpawnedComputer` (`/Game/Blueprints/AMJ-GameModeBase.AMJ_HoolProgressComponent` _asamj_game_mode_base)))

(event `self.ReceiveTick`
  (params (DeltaSeconds :type "Float (single-precision)"))
  (if (`self.IsDestroyed`)
    (bind _output_get (set `self.TimeToRespawn` (- (`self.TimeToRespawn`) DeltaSeconds)))
    (if (<= _output_get 0.0)
      (set `self.TimeToRespawn` 0.0)
      (`self.RespawnWorkStation`))))

(event `self.Box.OnComponentBeginOverlap`
  (params (OverlappedComponent :type "PrimitiveComponent Object Reference") (OtherActor :type "Actor Object Reference") (OtherComp :type "PrimitiveComponent Object Reference") (OtherBodyIndex :type Integer) (bFromSweep :type Boolean) (SweepResult :type "HitResult Structure (by ref)"))
  (`KismetSystemLibrary.PrintString` (`KismetSystemLibrary.GetDisplayName` OtherActor))
  (bind _asamj_programmer (cast `/Game/Blueprints/PlayableCharacters/AMJ-Programmer` OtherActor))
  (`/Game/Blueprints/PlayableCharacters/AMJ-Programmer.MakeCodingPossible` _asamj_programmer self))

(event `self.Box.OnComponentEndOverlap`
  (params (OverlappedComponent :type "PrimitiveComponent Object Reference") (OtherActor :type "Actor Object Reference") (OtherComp :type "PrimitiveComponent Object Reference") (OtherBodyIndex :type Integer))
  (`KismetSystemLibrary.PrintString` (`KismetSystemLibrary.GetDisplayName` OtherActor))
  (bind _asamj_programmer (cast `/Game/Blueprints/PlayableCharacters/AMJ-Programmer` OtherActor))
  (`/Game/Blueprints/PlayableCharacters/AMJ-Programmer.MakeCodingImpossible` _asamj_programmer))

(event `self.ReceiveAnyDamage`
  (params (Damage :type "Float (single-precision)") (DamageType :type "DamageType Object Reference") (InstigatedBy :type "Controller Object Reference") (DamageCauser :type "Actor Object Reference"))
  (`KismetSystemLibrary.PrintString` "Damage")
  (bind _output_get (set `self.Health` (- (`self.Health`) Damage)))
  (`self.SetHealthBar`)
  ;[1 0 0] WORKSTATION DEAD
  (if (<= _output_get 0.0)
    (`self.DestroyWorkStation`)))

(fn `DestroyWorkStation`
  (`|ExecutionSequence`
    (:`then_0`
      (bind _outactors (`GameplayStatics.GetAllActorsOfClass` "/Game/Blueprints/PlayableCharacters/AMJ-Programmer.AMJ-Programmer_C"))
      (for _array_element _outactors
        (`/Game/Blueprints/PlayableCharacters/AMJ-Programmer.OnDeskDestroyed` _array_element self)))
    (:`then_1`
      (`SceneComponent.SetVisibility` (`self.Desk`) false true)
      (`PrimitiveComponent.SetCollisionEnabled` (`self.Box`) "NoCollision")
      (`PrimitiveComponent.SetCollisionEnabled` (`self.Desk`) "NoCollision")
      (`PrimitiveComponent.SetCollisionEnabled` (`self.HitBox`) "NoCollision")
      (set `self.IsDestroyed` true)
      (set `self.TimeToRespawn` (`self.InitialTimeToRespawn`))
      (bind _asamj_game_mode_base (cast `/Game/Blueprints/AMJ-GameModeBase` (`GameplayStatics.GetGameMode`)))
      (`/Game/Blueprints/AMJ_HoolProgressComponent.OnComputerDestroy` (`/Game/Blueprints/AMJ-GameModeBase.AMJ_HoolProgressComponent` _asamj_game_mode_base))
      (`/Game/Blueprints/AMJ-Camera.Shake` (`/Game/Blueprints/AMJ-GameModeBase.Camera_Ref` _asamj_game_mode_base))
      (bind _returnvalue (`|SpawnActorFromClass` "/Game/Blueprints/AMJ-DestructibleWorkStation.AMJ-DestructibleWorkStation_C" (`KismetMathLibrary.MakeTransform` (.location (`self.GetTransform`)) (`KismetMathLibrary.MakeRotator` 0.0)) "Undefined" "OverrideRootScale"))
      (`/Game/Blueprints/AMJ-DestructibleWorkStation.Destroy` _returnvalue))
    (:`then_2`
      (`ActorComponent.SetActive` (`self.FX_BamEffect`) true true))))

(fn `RespawnWorkStation`
  (`SceneComponent.SetVisibility` (`self.Desk`) true true)
  (`PrimitiveComponent.SetCollisionEnabled` (`self.HitBox`) "QueryAndPhysics")
  (`PrimitiveComponent.SetCollisionEnabled` (`self.Box`) "QueryAndPhysics")
  (`PrimitiveComponent.SetCollisionEnabled` (`self.Desk`) "QueryAndPhysics")
  (set `self.IsDestroyed` false)
  (set `self.Health` (`self.MaxHealth`))
  (`self.SetHealthBar`)
  (bind _asamj_game_mode_base (cast `/Game/Blueprints/AMJ-GameModeBase` (`GameplayStatics.GetGameMode`)))
  (`/Game/Blueprints/AMJ_HoolProgressComponent.OnComputerRespawn` (`/Game/Blueprints/AMJ-GameModeBase.AMJ_HoolProgressComponent` _asamj_game_mode_base)))

(fn `SetHealthBar`
  (bind _ashpgui (cast `/Game/GUI/HPGUI` (`WidgetComponent.GetUserWidgetObject` (`self.HPBar`))))
  (`/Game/GUI/HPGUI.SetHP` _ashpgui (/ (`self.Health`) (`self.MaxHealth`))))

(fn `UserConstructionScript`
  (`SceneComponent.K2_SetRelativeRotation` (`self.Desk`) (`KismetMathLibrary.MakeRotator` 0.0 0.0 (`self.Rotation`)) false false))