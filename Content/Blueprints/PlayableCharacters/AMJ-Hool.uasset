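; AMJ-Hool is a playable character that attacks workstations and, when allowed, programmers.
; Hit input, unless frozen, runs a forward line trace that damages workstations by Strength and notifies the game mode's ProdSystem.
; Too many programmer hits trigger game over, while a child-actor sound controller plays hit or swing sounds.
; Tick counts down an attack timer gating walking and attack animation, and shows a billboard when facing a workstation in range.
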(event `InputAction|Hit`
  (params (Key :type "Key Structure" :default "AnyKey"))
  (:`Pressed`
    (if (not (`self.IsFrozen`))
      (`self.UseWeapon`))))

(event `self.ReceiveTick`
  (params (DeltaSeconds :type "Float (single-precision)"))
  (`|ExecutionSequence`
    (:`then_0`
      (if (> (`self.AttackTimer`) 0.0)
        (set `self.AttackTimer` (- (`self.AttackTimer`) DeltaSeconds))))
    (:`then_1`
      (bind _outhit (`KismetSystemLibrary.LineTraceSingle` (`self.K2_GetActorLocation`) (+ (`self.K2_GetActorLocation`) (* (`self.GetActorForwardVector`) 300.0)) "TraceTypeQuery1"))
      (cast `/Game/Blueprints/AMJWorkstation` (`.HitActor` (`GameplayStatics.BreakHitResult` _outhit))
        (:`then`
          (`SceneComponent.SetVisibility` (`self.Billboard`) true false))
        (:`CastFailed`
          (`SceneComponent.SetVisibility` (`self.Billboard`) false false))))))

(fn `AttackAnimShouldBePlayed`
  (returns (Should :type Boolean))
  (return (> (`self.AttackTimer`) 0.0)))

(fn `CanWalk`
  (returns (CanWalk :type Boolean))
  (return (<= (`self.AttackTimer`) 0.0)))

(fn `GetSoundControler`
  (returns (OutSoundControler :type "/Game/Blueprints/PlayableCharacters/AMJ-SoundControlHool Object Reference"))
  (bind _asamj_sound_control_hool (cast `/Game/Blueprints/PlayableCharacters/AMJ-SoundControlHool` (`ChildActorComponent.ChildActor` (`self.SoundControler`))))
  (return _asamj_sound_control_hool))

(fn `UserConstructionScript`)

(fn `UseWeapon`
  (set `self.AttackTimer` 0.2)
  (bind _outhit (`KismetSystemLibrary.LineTraceSingle` (`self.K2_GetActorLocation`) (+ (`self.K2_GetActorLocation`) (* (`self.GetActorForwardVector`) 300.0)) "TraceTypeQuery1"))
  (if (`GameplayStatics.BreakHitResult` _outhit)
    (bind _asamjworkstation (cast `/Game/Blueprints/AMJWorkstation` (`.HitActor` (`GameplayStatics.BreakHitResult` _outhit)))
      (:`then`
        (`GameplayStatics.ApplyDamage` _asamjworkstation (`self.Strength`) null self)
        (`/Game/Blueprints/PlayableCharacters/AMJ-SoundControlHool.PlayHit` (`self.GetSoundControler`))
        (`/Game/Blueprints/ProdAndTrust/ProdSystemComponent.AttackPerformed` (`self.GetComponentByClass` (`GameplayStatics.GetGameMode`) "/Game/Blueprints/ProdAndTrust/ProdSystemComponent.ProdSystemComponent_C")))
      (:`CastFailed`
        (if (`self.CanHitProgrammer`)
          (cast `/Game/Blueprints/PlayableCharacters/AMJ-Programmer` (`.HitActor` (`GameplayStatics.BreakHitResult` _outhit))
            (:`then`
              (`/Engine/EditorBlueprintResources/StandardMacros.IncrementInt` (`self.CurrentProgrammerHit`)
                (:`  `
                  (if (> (`self.CurrentProgrammerHit`) (`self.MaxProgrammerHit`))
                    (bind _asamj_game_mode_base (cast `/Game/Blueprints/AMJ-GameModeBase` (`GameplayStatics.GetGameMode`))
                      (:`then`
                        (`/Game/Blueprints/AMJ-GameModeBase.GameOver` _asamj_game_mode_base false true))
                      (:`CastFailed`
                        (`/Game/Blueprints/PlayableCharacters/AMJ-SoundControlHool.PlaySwing` (`self.GetSoundControler`) :!label _label)))
                    (else
                      (`/Game/Blueprints/PlayableCharacters/AMJ-SoundControlHool.PlayHit` (`self.GetSoundControler`)))))))
            (:`CastFailed`
              (goto _label))))))
    (else
      (`/Game/Blueprints/PlayableCharacters/AMJ-SoundControlHool.PlaySwing` (`self.GetSoundControler`)))))