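; Sound control Blueprint for the Programmer playable character, providing audio cues for keyboard hits, getting a task, failing and completing.
; Each cue is a separate function that plays its own audio component from the start.
; Keyboard and fail sounds skip playback if already playing, while the get-task and complete sounds play on every call.
; It has no active event logic or construction logic.
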(fn `PlayComplete`
  (`AudioComponent.Play` (`self.CompleteSound`) 0.0))

(fn `PlayFail`
  (bind _failsound (`self.FailSound`))
  (if (not (`AudioComponent.IsPlaying` _failsound))
    (`AudioComponent.Play` _failsound 0.0)))

(fn `PlayGetTask`
  (`AudioComponent.Play` (`self.GetTaskSound`) 0.0))

(fn `PlayKeyboardSound`
  (bind _keyboardhitsound (`self.KeyboardHitSound`))
  (if (not (`AudioComponent.IsPlaying` _keyboardhitsound))
    (`AudioComponent.Play` _keyboardhitsound 0.0)))

(fn `UserConstructionScript`)