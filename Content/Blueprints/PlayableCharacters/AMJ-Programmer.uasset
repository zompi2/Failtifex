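; Playable programmer character that picks up tasks at boards and codes at workstations to complete them.
; A state variable routes the Code input to picking or coding, with billboards showing what is possible.
; Tasks and progress live in the GameMode's progress component, whose finished event triggers spawning the next task.
; Each press adds progress and restarts a short timer that drives animation, blocks walking and flags interruption if the desk is destroyed.
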(event `InputAction|Code`
  (params (Key :type "Key Structure" :default "AnyKey"))
  ;[1 1 1] Action
  (:`Pressed`
    (switch `/Game/Blueprints/PlayableCharacters/AMJ-ProgrammerState` (`self.CurrentState`)
      (:`NewEnumerator1`
        (`self.PickTask`))
      (:`NewEnumerator2`
        (`self.Code`)))))

(event `self.ReceiveBeginPlay`
  ;[1 1 1] Binding Event for finishing coding task
  (bind _asamj_game_mode_base (cast `/Game/Blueprints/AMJ-GameModeBase` (`GameplayStatics.GetGameMode`)))
  (add `/Game/Blueprints/AMJ_ProgressComponent.OnFinishedEvent` (`/Game/Blueprints/AMJ-GameModeBase.AMJ_ProgressComponent` _asamj_game_mode_base) (delegate `OnFinishedTask`))
  (`self.SetCodeProgress` 0.0))

(event `OnFinishedTask`
  ;[1 1 1] Binding Event for finishing coding task
  (`self.FinishedTask`))

(event `self.ReceiveTick`
  (params (DeltaSeconds :type "Float (single-precision)"))
  (if (> (`self.CodingTimer`) 0.0)
    (bind _output_get (set `self.CodingTimer` (- (`self.CodingTimer`) DeltaSeconds)))
    (if (<= _output_get 0.0)
      (set `self.CodingWasInterupted` false))))

(fn `CanWalk`
  (returns (CanWalk :type Boolean))
  (return (<= (`self.CodingTimer`) 0.0)))

(fn `Code`
  (locals (CodeProgressPercent :type "Float (double-precision)" :default 0.0))
  (bind _currentworkstation (`self.CurrentWorkstation`))
  (`/Engine/EditorBlueprintResources/StandardMacros.IsValid` _currentworkstation
    (:`Is Valid`
      (`self.K2_SetActorRotation` (`KismetMathLibrary.MakeRotator` 0.0 0.0 (`/Game/Blueprints/AMJWorkstation.Rotation` _currentworkstation))))
    (:`Is Not Valid`
      _))
  (bind _asamj_game_mode_base (cast `/Game/Blueprints/AMJ-GameModeBase` (`GameplayStatics.GetGameMode`)))
  (bind _amj_progresscomponent (`/Game/Blueprints/AMJ-GameModeBase.AMJ_ProgressComponent` _asamj_game_mode_base))
  (if (`/Game/Blueprints/AMJ_ProgressComponent.HasActiveTask` _amj_progresscomponent)
    (`KismetSystemLibrary.PrintString` "I'm coding!")
    (set `self.CodingTimer` 0.2)
    (`/Game/Blueprints/PlayableCharacters/AMJ-SoundControl-Programmer.PlayKeyboardSound` (`self.GetSoundController`))
    (bind _progresspercent (`/Game/Blueprints/AMJ_ProgressComponent.AddProgress` _amj_progresscomponent (`self.CodingPower`)))
    (set `local.CodeProgressPercent` _progresspercent)
    (bind _ascode_gui (cast `/Game/GUI/CodeGUI` (`WidgetComponent.GetUserWidgetObject` (`self.CodeBar`))))
    (`/Game/GUI/CodeGUI.SetCodeProgress` _ascode_gui (`local.CodeProgressPercent`))
    (else
      (`KismetSystemLibrary.PrintString` "Can't code without task!")
      (`/Game/Blueprints/PlayableCharacters/AMJ-SoundControl-Programmer.PlayFail` (`self.GetSoundController`)))))

(fn `FinishedTask`
  (`self.MakeCodingImpossible`)
  (`SceneComponent.SetVisibility` (`self.DoneBill`) true false)
  (`/Game/Blueprints/PlayableCharacters/AMJ-SoundControl-Programmer.PlayComplete` (`self.GetSoundController`))
  (bind _asamj_game_mode_base (cast `/Game/Blueprints/AMJ-GameModeBase` (`GameplayStatics.GetGameMode`)))
  (`/Game/Blueprints/AMJ_ProgressComponent.SpawnNextTask` (`/Game/Blueprints/AMJ-GameModeBase.AMJ_ProgressComponent` _asamj_game_mode_base)))

(fn `GetSoundController`
  (returns (OutSoundController :type "/Game/Blueprints/PlayableCharacters/AMJ-SoundControl-Programmer Object Reference"))
  (bind _asamj_sound_control__programmer (cast `/Game/Blueprints/PlayableCharacters/AMJ-SoundControl-Programmer` (`ChildActorComponent.ChildActor` (`self.SoundControllerActor`))))
  (return _asamj_sound_control__programmer))

(fn `MakeCodingImpossible`
  (`SceneComponent.SetVisibility` (`self.DoneBill`) false false)
  (if (`|EnumEquality` (`self.CurrentState`) "NewEnumerator2")
    (set `self.CurrentState` "NewEnumerator0")
    (`SceneComponent.SetVisibility` (`self.CodeBill`) false false)
    (`SceneComponent.SetVisibility` (`self.NoTask`) false false)))

(fn `MakeCodingPossible`
  (params (InWorkstation :type "/Game/Blueprints/AMJWorkstation Object Reference"))
  (set `self.CurrentWorkstation` InWorkstation)
  (if (`|EnumEquality` (`self.CurrentState`) "NewEnumerator0")
    (set `self.CurrentState` "NewEnumerator2")
    (bind _asamj_game_mode_base (cast `/Game/Blueprints/AMJ-GameModeBase` (`GameplayStatics.GetGameMode`)))
    (if (`/Game/Blueprints/AMJ_ProgressComponent.HasActiveTask` (`/Game/Blueprints/AMJ-GameModeBase.AMJ_ProgressComponent` _asamj_game_mode_base))
      (`SceneComponent.SetVisibility` (`self.CodeBill`) true false)
      (`KismetSystemLibrary.PrintString` "CAN CODING")
      (else
        (`SceneComponent.SetVisibility` (`self.NoTask`) true false)
        (`KismetSystemLibrary.PrintString` "NO TASK!")))))

(fn `OnDeskDestroyed`
  (params (Workstation :type "/Game/Blueprints/AMJWorkstation Object Reference"))
  (if (and (== Workstation (`self.CurrentWorkstation`)) (> (`self.CodingTimer`) 0.0))
    (set `self.CodingWasInterupted` true)))

(fn `PickTask`
  (bind _asamj_game_mode_base (cast `/Game/Blueprints/AMJ-GameModeBase` (`GameplayStatics.GetGameMode`)))
  (bind _amj_progresscomponent (`/Game/Blueprints/AMJ-GameModeBase.AMJ_ProgressComponent` _asamj_game_mode_base))
  (if (`/Game/Blueprints/AMJ_ProgressComponent.HasActiveTask` _amj_progresscomponent)
    (`KismetSystemLibrary.PrintString` "ALREADY HAS A TASK")
    (`/Game/Blueprints/PlayableCharacters/AMJ-SoundControl-Programmer.PlayFail` (`self.GetSoundController`))
    (else
      (`/Game/Blueprints/AMJ_ProgressComponent.LaunchTask` _amj_progresscomponent (`/Game/Blueprints/AMJ-Board.TaskId` (`self.CheckingBoard`)))
      (`self.SetCodeProgressColor` (`/Game/Blueprints/AMJ-Board.Color` (`self.CheckingBoard`)))
      (`/Game/Blueprints/AMJ-Board.OnPickedUp` (`self.CheckingBoard`))
      (`self.StopPickingNewTask`)
      (`/Game/Blueprints/PlayableCharacters/AMJ-SoundControl-Programmer.PlayGetTask` (`self.GetSoundController`)))))

(fn `SetCodeProgress`
  (params (InProgress :type "Float (double-precision)"))
  (bind _ascode_gui (cast `/Game/GUI/CodeGUI` (`WidgetComponent.GetUserWidgetObject` (`self.CodeBar`))))
  (`/Game/GUI/CodeGUI.SetCodeProgress` _ascode_gui InProgress))

(fn `SetCodeProgressColor`
  (params (InColor :type "LinearColor Structure"))
  (bind (_r _g _b) (break `LinearColor` InColor))
  (bind _ascode_gui (cast `/Game/GUI/CodeGUI` (`WidgetComponent.GetUserWidgetObject` (`self.CodeBar`))))
  (`ProgressBar.SetFillColorAndOpacity` (`/Game/GUI/CodeGUI.ProgressBar_34` _ascode_gui) (make `LinearColor` _r _g _b 1.0)))

(fn `ShouldPlayCodingAnim`
  (returns (Should :type Boolean))
  (return (> (`self.CodingTimer`) 0.0)))

(fn `StartPickingNewTask`
  (params (InBoard :type "/Game/Blueprints/AMJ-Board Object Reference"))
  (set `self.CheckingBoard` InBoard)
  (if (`|EnumEquality` (`self.CurrentState`) "NewEnumerator0")
    (set `self.CurrentState` "NewEnumerator1")
    (bind _asamj_game_mode_base (cast `/Game/Blueprints/AMJ-GameModeBase` (`GameplayStatics.GetGameMode`)))
    (if (`/Game/Blueprints/AMJ_ProgressComponent.HasActiveTask` (`/Game/Blueprints/AMJ-GameModeBase.AMJ_ProgressComponent` _asamj_game_mode_base))
      (`SceneComponent.SetVisibility` (`self.FinishTask`) true false)
      (`KismetSystemLibrary.PrintString` "PICKING TASK, ALREADY HS")
      (else
        (`SceneComponent.SetVisibility` (`self.PickTaskBill`) true false)
        (`KismetSystemLibrary.PrintString` "PICKING TASK")))))

(fn `StopPickingNewTask`
  (if (`|EnumEquality` (`self.CurrentState`) "NewEnumerator1")
    (set `self.CurrentState` "NewEnumerator0")
    (`SceneComponent.SetVisibility` (`self.PickTaskBill`) false false)
    (`SceneComponent.SetVisibility` (`self.FinishTask`) false false)
    (`KismetSystemLibrary.PrintString` "FINISHED PICKING TASK")))

(fn `UserConstructionScript`)