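; Task board actor that offers a task for an AMJ-Programmer to pick up.
; Overlapping its box starts the programmer picking the task, and leaving stops it.
; OnPickedUp hides the board and disables collision; RespawnBoard pulls the next task ID from the game mode's progress component and, if one exists, restores the board.
; Each respawn tints the board with the task's color through a dynamic material instance.
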(event `self.Box.OnComponentBeginOverlap`
  (params (OverlappedComponent :type "PrimitiveComponent Object Reference") (OtherActor :type "Actor Object Reference") (OtherComp :type "PrimitiveComponent Object Reference") (OtherBodyIndex :type Integer) (bFromSweep :type Boolean) (SweepResult :type "HitResult Structure (by ref)"))
  (bind _asamj_programmer (cast `/Game/Blueprints/PlayableCharacters/AMJ-Programmer` OtherActor))
  (`/Game/Blueprints/PlayableCharacters/AMJ-Programmer.StartPickingNewTask` _asamj_programmer self)
  (bind _asamj_game_mode_base (cast `/Game/Blueprints/AMJ-GameModeBase` (`GameplayStatics.GetGameMode`))))

(event `self.Box.OnComponentEndOverlap`
  (params (OverlappedComponent :type "PrimitiveComponent Object Reference") (OtherActor :type "Actor Object Reference") (OtherComp :type "PrimitiveComponent Object Reference") (OtherBodyIndex :type Integer))
  (bind _asamj_programmer (cast `/Game/Blueprints/PlayableCharacters/AMJ-Programmer` OtherActor))
  (`/Game/Blueprints/PlayableCharacters/AMJ-Programmer.StopPickingNewTask` _asamj_programmer))

(fn `GetMainGUIWidget`
  (returns (Out :type "/Game/GUI/MainGUI Object Reference"))
  (bind _asamj_game_mode_base (cast `/Game/Blueprints/AMJ-GameModeBase` (`GameplayStatics.GetGameMode`)))
  (return (`/Game/Blueprints/AMJ-GameModeBase.MainGUI_Ref` _asamj_game_mode_base)))

(fn `OnPickedUp`
  (set `self.IsPickedUp` true)
  (`SceneComponent.SetVisibility` (`self.Scene`) false true)
  (`PrimitiveComponent.SetCollisionEnabled` (`self.Box`) "NoCollision"))

(fn `RespawnBoard`
  (bind _asamj_game_mode_base (cast `/Game/Blueprints/AMJ-GameModeBase` (`GameplayStatics.GetGameMode`)))
  (bind _amj_progresscomponent (`/Game/Blueprints/AMJ-GameModeBase.AMJ_ProgressComponent` _asamj_game_mode_base))
  (bind _outid (`/Game/Blueprints/AMJ_ProgressComponent.GetNextTask` _amj_progresscomponent))
  (if (not (== _outid -1))
    (`SceneComponent.SetVisibility` (`self.Scene`) true true)
    (`PrimitiveComponent.SetCollisionEnabled` (`self.Box`) "QueryAndPhysics")
    (set `self.TaskId` _outid)
    (bind (_id _tasktitle _tasktext _progresstomake _reward _color _scale) (break `/Game/Blueprints/AMJ-TasksData` (`BlueprintMapLibrary.Map_Find` (`/Game/Blueprints/AMJ_ProgressComponent.Tasks` _amj_progresscomponent) (`self.TaskId`))))
    (set `self.Color` _color)
    (`self.SetMaterialColor` _color)
    (set `self.IsPickedUp` false)))

(fn `SetMaterialColor`
  (params (InColor :type "LinearColor Structure"))
  (bind _returnvalue (`PrimitiveComponent.CreateDynamicMaterialInstance` (`self.Cube`) 0 "/Game/Blueprints/BoardMaterialInstance.BoardMaterialInstance"))
  (`MaterialInstanceDynamic.SetVectorParameterValue` _returnvalue "color" InColor))

(fn `UserConstructionScript`)