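; Progress component that runs the game's task loop, tracking the active task and overall progress toward winning.
; BeginPlay fills an ID-keyed map with hard-coded placeholder tasks, which GetNextTask hands out via TasksOrder.
; Added progress completes the launched task, banking its reward, updating the GUI, briefly showing a random programmer message and firing a finished event.
; Spawned boards' rewards raise the overall target; reaching it calls GameOver on the game mode.
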(event `self.ReceiveBeginPlay`
  (`self.SetUpTasks`))

(event `HideMessage`
  (bind _asamj_game_mode_base (cast `/Game/Blueprints/AMJ-GameModeBase` (`GameplayStatics.GetGameMode`)))
  (`/Game/GUI/MainGUI.HideProgrammerMessage` (`/Game/Blueprints/AMJ-GameModeBase.MainGUI_Ref` _asamj_game_mode_base) ""))

(fn `AddNewTsk`
  (params (Title :type Text) (Text :type Text) (ProgressToMake :type "Float (double-precision)") (Id :type Integer) (Reward :type "Float (double-precision)") (Color :type "LinearColor Structure") (Scale :type "Vector2D Structure" :default (1.0 0.0)))
  (`BlueprintMapLibrary.Map_Add` (`self.Tasks`) Id (make `/Game/Blueprints/AMJ-TasksData` Id Title Text ProgressToMake Reward Color Scale)))

(fn `AddProgress`
  (params (ProgressToAdd :type "Float (double-precision)"))
  (returns (ProgressPercent :type "Float (double-precision)"))
  (if (`self.HasActiveTask`)
    (bind _output_get (set `self.Progress` (+ (`self.Progress`) ProgressToAdd)))
    (`KismetSystemLibrary.PrintString` (`KismetStringLibrary.Concat_StrStr` "Progress: " (`KismetStringLibrary.Conv_DoubleToString` _output_get) " / " (`KismetStringLibrary.Conv_DoubleToString` (`self.RequiredProgress`))))
    (`self.ProcessProgress`)
    (return (/ (`self.Progress`) (`self.RequiredProgress`)))))

(fn `FinishedTask`
  (`|ExecutionSequence`
    (:`then_0`
      (bind _asamj_game_mode_base (cast `/Game/Blueprints/AMJ-GameModeBase` (`GameplayStatics.GetGameMode`)))
      (`/Game/GUI/MainGUI.ShowProgrammerMessage` (`/Game/Blueprints/AMJ-GameModeBase.MainGUI_Ref` _asamj_game_mode_base) (`|GetArrayItem` (`self.Messages`) (`KismetMathLibrary.RandomIntegerInRange` 0 (- (`KismetArrayLibrary.Array_Length` (`self.Messages`)) 1))))
      (`KismetSystemLibrary.K2_SetTimerDelegate` (`|CreateDelegate` :!event `HideMessage`) 4.0))
    (:`then_1`
      ;[1 1 1] Add to overall progress
      (set `self.CurrentOverallProgress` (+ (`self.CurrentOverallProgress`) (`self.PendingReward`)))
      ;[1 1 1] Update the progress bar
      (bind _asamj_game_mode_base_2 (cast `/Game/Blueprints/AMJ-GameModeBase` (`GameplayStatics.GetGameMode`)))
      (`/Game/GUI/MainGUI.UpdateProgress` (`/Game/Blueprints/AMJ-GameModeBase.MainGUI_Ref` _asamj_game_mode_base_2) (/ (* (`self.CurrentOverallProgress`) 100.0) (`self.OverallProgress`)))
      ;[1 1 1] Clear fields
      (set `self.RequiredProgress` 0.0)
      (set `self.Progress` 0.0)
      (set `self.PendingReward` 0.0)
      (set `self.HasActiveTask` false)
      (`self.OnFinishedEvent`)
      (`KismetSystemLibrary.PrintString` "FINISHED TASK!")
      ;[1 1 1] Check if make game over
      (if (>= (`self.CurrentOverallProgress`) (`self.OverallProgress`))
        (bind _asamj_game_mode_base_3 (cast `/Game/Blueprints/AMJ-GameModeBase` (`GameplayStatics.GetGameMode`)))
        (`/Game/Blueprints/AMJ-GameModeBase.GameOver` _asamj_game_mode_base_3 true)))))

(fn `GetNextTask`
  (returns (OutId :type Integer))
  (locals (LocalOut :type Integer))
  (if (== (`KismetArrayLibrary.Array_Length` (`self.TasksOrder`)) (`self.LastPicketOrderIdx`))
    (return -1)
    (else
      (set `local.LocalOut` (`|GetArrayItem` (`self.TasksOrder`) (`self.LastPicketOrderIdx`)))
      (`/Engine/EditorBlueprintResources/StandardMacros.IncrementInt` (`self.LastPicketOrderIdx`)
        (:`  `
          (return (`local.LocalOut`)))))))

(fn `LaunchTask`
  (params (Id :type Integer))
  (bind (_id _tasktitle _tasktext _progresstomake _reward) (break `/Game/Blueprints/AMJ-TasksData` (`BlueprintMapLibrary.Map_Find` (`self.Tasks`) (`self.CurrentTaskId`))))
  (set `self.CurrentTaskId` Id)
  (set `self.HasActiveTask` true)
  (`KismetSystemLibrary.PrintString` "LAUNCHING TASK")
  (`KismetSystemLibrary.PrintString` (`KismetStringLibrary.Conv_IntToString` Id))
  (`KismetSystemLibrary.PrintText` _tasktitle)
  (`KismetSystemLibrary.PrintText` _tasktext)
  (`KismetSystemLibrary.PrintString` (`KismetStringLibrary.Conv_DoubleToString` _progresstomake))
  (set `self.RequiredProgress` _progresstomake)
  (set `self.PendingReward` _reward))

(fn `OnSpawnedNewBoard`
  (params (InBoard :type "/Game/Blueprints/AMJ-Board Object Reference"))
  (set `self.OverallProgress` (+ (`self.OverallProgress`) (`.Reward_20_883C43E543D1ADDAEACAE6BBD3C25E35` (break `/Game/Blueprints/AMJ-TasksData` (`BlueprintMapLibrary.Map_Find` (`self.Tasks`) (`/Game/Blueprints/AMJ-Board.TaskId` InBoard)))))))

(fn `ProcessProgress`
  (if (>= (`self.Progress`) (`self.RequiredProgress`))
    (`self.FinishedTask`)
    (elif (< (`self.Progress`) 0.0)
      (set `self.Progress` 0.0))))

(fn `RemoveProgress`
  (params (ProgressToRemove :type "Float (double-precision)"))
  (if (`self.HasActiveTask`)
    (set `self.Progress` (- (`self.Progress`) ProgressToRemove))
    (`self.ProcessProgress`)))

(fn `SetUpTasks`
  (locals (green :type "LinearColor Structure" :default (struct :`R` 0.021182 :`G` 0.37)) (yellow :type "LinearColor Structure" :default (struct :`R` 1.0 :`G` 0.478997)) (red :type "LinearColor Structure" :default (struct :`R` 1.0 :`G` 0.009744)))
  (`self.AddNewTsk` "Another Task" "Some Description" 60.0 101 40.0 (`local.green`) (1.0 1.0))
  (`self.AddNewTsk` "Another Task 2" "Some Description 2" 60.0 102 40.0 (`local.green`) (1.0 1.0))
  (`self.AddNewTsk` "Another Task 2" "Some Description 2" 75.0 203 60.0 (`local.yellow`) (1.0 1.0))
  (`self.AddNewTsk` "Another Task 2" "Some Description 2" 90.0 304 90.0 (`local.red`) (1.0 1.0))
  (`self.AddNewTsk` "Another Task 2" "Some Description 2" 60.0 105 40.0 (`local.green`) (1.0 1.0))
  (`self.AddNewTsk` "Another Task 2" "Some Description 2" 75.0 206 60.0 (`local.yellow`) (1.0 1.0))
  (`self.AddNewTsk` "Another Task 2" "Some Description 2" 90.0 307 90.0 (`local.red`) (1.0 1.0))
  (`self.AddNewTsk` "Another Task 2" "Some Description 2" 60.0 108 45.0 (`local.green`) (1.0 1.0))
  (`self.AddNewTsk` "Another Task 2" "Some Description 2" 60.0 109 45.0 (`local.green`) (1.0 1.0))
  (`self.AddNewTsk` "Another Task 2" "Some Description 2" 75.0 210 60.0 (`local.yellow`) (1.0 1.0))
  (`self.AddNewTsk` "Another Task 2" "Some Description 2" 90.0 311 90.0 (`local.red`) (1.0 1.0))
  (`self.AddNewTsk` "Another Task 2" "Some Description 2" 75.0 212 60.0 (`local.yellow`) (1.0 1.0))
  (`self.AddNewTsk` "Another Task 2" "Some Description 2" 60.0 113 45.0 (`local.green`) (1.0 1.0))
  (`self.AddNewTsk` "Another Task 2" "Some Description 2" 60.0 114 45.0 (`local.green`) (1.0 1.0))
  (`self.AddNewTsk` "Another Task 2" "Some Description 2" 90.0 315 90.0 (`local.red`) (1.0 1.0))
  (`self.AddNewTsk` "Another Task 2" "Some Description 2" 90.0 316 90.0 (`local.red`) (1.0 1.0)))

(fn `SpawnNextTask`
  (bind _outactors (`GameplayStatics.GetAllActorsOfClass` "/Game/Blueprints/AMJ-Board.AMJ-Board_C"))
  (for _array_element _outactors
    (if (`/Game/Blueprints/AMJ-Board.IsPickedUp` _array_element)
      (`/Game/Blueprints/AMJ-Board.RespawnBoard` _array_element))))