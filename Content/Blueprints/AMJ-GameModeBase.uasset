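; Game mode for a two-player local match between a Programmer and a Hool, handling setup, round timer and game over.
; Spawns pawn classes by player count and points a shared camera at both characters, or at the Programmer and Producer.
; StartLevel creates the GUI, starts music and respawns boards; Tick counts down the round, with timeout a Hool win.
; GameOver stores the outcome in the game instance, then opens GameOverScreen.
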(event `self.ReceiveTick`
  (params (DeltaSeconds :type "Float (single-precision)"))
  (`self.TickSprintTime` DeltaSeconds))

(fn `GameOver`
  (params (bDidProgrammerWon :type Boolean) (bDidProgrammerBeignHit :type Boolean))
  (bind _returnvalue (`GameplayStatics.GetGameInstance`))
  (if bDidProgrammerBeignHit
    (set `self.EGameState` "NewEnumerator4")
    (`KismetSystemLibrary.PrintString` "GAME OVER PROGRAMMER DEAD")
    (bind _asamj_game_instance (cast `/Game/Blueprints/AMJ-GameInstance` _returnvalue))
    (set `/Game/Blueprints/AMJ-GameInstance.bDidProgrammerDead` true _asamj_game_instance)
    (else
      (if bDidProgrammerWon
        (set `self.EGameState` "NewEnumerator2")
        (`KismetSystemLibrary.PrintString` "GAME OVER PROGRAMMER WON")
        (bind _asamj_game_instance_2 (cast `/Game/Blueprints/AMJ-GameInstance` (`GameplayStatics.GetGameInstance`)))
        (set `/Game/Blueprints/AMJ-GameInstance.bDidProgrammerWon` true _asamj_game_instance_2)
        (else
          (set `self.EGameState` "NewEnumerator3")
          (`KismetSystemLibrary.PrintString` "GAME OVER HOOL WON")
          (bind _asamj_game_instance_3 (cast `/Game/Blueprints/AMJ-GameInstance` _returnvalue))
          (set `/Game/Blueprints/AMJ-GameInstance.bDidProgrammerWon` false _asamj_game_instance_3)))
      (bind _asamj_game_instance_4 (cast `/Game/Blueprints/AMJ-GameInstance` (`GameplayStatics.GetGameInstance`)))
      (set `/Game/Blueprints/AMJ-GameInstance.bDidProgrammerDead` false _asamj_game_instance_4)))
  (`GameplayStatics.OpenLevel` "GameOverScreen"))

(fn `SetCharactersToCamera`
  (locals (ProgrammerActor :type "/Game/Blueprints/PlayableCharacters/AMJ-Programmer Object Reference") (`Hool Actor` :type "/Game/Blueprints/PlayableCharacters/AMJ-Hool Object Reference"))
  (bind _outactors (`GameplayStatics.GetAllActorsOfClass` "/Game/Blueprints/PlayableCharacters/AMJ-Programmer.AMJ-Programmer_C"))
  (set `local.ProgrammerActor` (`|GetArrayItem` _outactors))
  (bind _outactors_2 (`GameplayStatics.GetAllActorsOfClass` "/Game/Blueprints/PlayableCharacters/AMJ-Hool.AMJ-Hool_C"))
  (set `local.Hool Actor` (`|GetArrayItem` _outactors_2))
  (`/Game/Blueprints/AMJ-Camera.SetPlayersToCamera` (`self.Camera_Ref`) (`local.ProgrammerActor`) (`local.Hool Actor`)))

(fn `SetProducerToCamera`
  (locals (`Prod Actor` :type "/Game/Blueprints/ProdAndTrust/AMJ_Prod Object Reference") (`Programmer Actor` :type "/Game/Blueprints/PlayableCharacters/AMJ_Character Object Reference"))
  (bind _outactors (`GameplayStatics.GetAllActorsOfClass` "/Game/Blueprints/PlayableCharacters/AMJ-Programmer.AMJ-Programmer_C"))
  (set `local.Programmer Actor` (`|GetArrayItem` _outactors))
  (bind _outactors_2 (`GameplayStatics.GetAllActorsOfClass` "/Game/Blueprints/ProdAndTrust/AMJ_Prod.AMJ_Prod_C"))
  (set `local.Prod Actor` (`|GetArrayItem` _outactors_2))
  (`/Game/Blueprints/AMJ-Camera.SetPlayersToCamera` (`self.Camera_Ref`) (`local.Programmer Actor`) (`local.Prod Actor`)))

(fn `SpawnDefaultPawnFor`
  (params (NewPlayer :type "Controller Object Reference") (StartSpot :type "Actor Object Reference"))
  (returns (ReturnValue :type "Pawn Object Reference"))
  (locals (SpawnedCharacter :type "/Game/Blueprints/PlayableCharacters/AMJ_Character Object Reference"))
  (bind _returnvalue (`self.GetNumPlayers`))
  (bind _returnvalue_2 (`|SpawnActorFromClass` (`|GetArrayItem` (`self.PlayerClasses`) (- _returnvalue 1)) (`KismetMathLibrary.Conv_VectorToTransform` (`self.K2_GetActorLocation` StartSpot)) "AlwaysSpawn" "OverrideRootScale"))
  (set `local.SpawnedCharacter` _returnvalue_2)
  (`|ExecutionSequence`
    (:`then_0`
      ;[1 1 1] Add player to camera if camera ref exists
      (if (`KismetSystemLibrary.IsValid` (`self.Camera_Ref`))
        (`self.SetCharactersToCamera`)))
    (:`then_1`
      (return (`local.SpawnedCharacter`)))))

(fn `StartLevel`
  ;[1 1 1] Get Camera Ref
  (bind _outactors (`GameplayStatics.GetAllActorsOfClass` "/Game/Blueprints/AMJ-Camera.AMJ-Camera_C"))
  (bind _output_get (set `self.Camera_Ref` (`|GetArrayItem` _outactors)))
  (`/Game/Blueprints/AMJ-Camera.SetThisCameraToViewport` _output_get)
  (`self.SetCharactersToCamera`)
  ;[1 1 1] Create and save GUI
  (bind _returnvalue (`|CreateWidget` "/Game/GUI/MainGUI.MainGUI_C"))
  (bind _output_get_2 (set `self.MainGUI_Ref` _returnvalue))
  (`UserWidget.AddToViewport` _output_get_2 0)
  ;[1 1 1] Get Music Controller and Play it
  (bind _outactors_2 (`GameplayStatics.GetAllActorsOfClass` "/Game/Blueprints/AMJ-MusicController.AMJ-MusicController_C"))
  (bind _output_get_3 (set `self.Music_Ref` (`|GetArrayItem` _outactors_2)))
  (`/Game/Blueprints/AMJ-MusicController.Play` _output_get_3)
  ;[1 1 1] Refresh first three boards
  (bind _outactors_3 (`GameplayStatics.GetAllActorsOfClass` "/Game/Blueprints/AMJ-Board.AMJ-Board_C"))
  (for _array_element _outactors_3
    (`/Game/Blueprints/AMJ-Board.RespawnBoard` _array_element)))

(fn `TickSprintTime`
  (params (DeltaTime :type "Float (double-precision)"))
  (bind _maingui_ref (`self.MainGUI_Ref`))
  (if (`self.IsTicking`)
    (if (`|EnumEquality` (`self.EGameState`) "NewEnumerator1")
      (bind _output_get (set `self.RoundTime` (- (`self.RoundTime`) DeltaTime)))
      (if (< _output_get 1.0)
        (`/Game/GUI/MainGUI.UpdateTime` (`self.MainGUI_Ref`) 0)
        (`self.GameOver` false)
        (else
          (`/Engine/EditorBlueprintResources/StandardMacros.IsValid` _maingui_ref
            (:`Is Valid`
              (`/Game/GUI/MainGUI.UpdateTime` _maingui_ref (`KismetMathLibrary.FTrunc` _output_get)))))))))

(fn `UserConstructionScript`)