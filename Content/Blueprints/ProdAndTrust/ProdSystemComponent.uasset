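; Component that runs a trust meter and spawns a "Prod" AI actor whenever trust runs out.
; While trusting, Trust drains each tick and with every attack; at zero the Prod spawns at the first tagged spawn point.
; While it is out, attacks set its WasNaughty blackboard key according to whether it is stationary.
; Once the Prod finishes, it is destroyed and Trust resets with a new random drain speed.
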(event `self.ReceiveTick`
  (params (DeltaSeconds :type "Float (single-precision)"))
  (bind (_trustspeedrange_x _trustspeedrange_y) (`KismetMathLibrary.BreakVector2D` (`self.TrustSpeedRange`)))
  (if (`self.IsProdTrusting`)
    (`self.DecreaseTrust` (* DeltaSeconds (`self.TrustLooseSpeed`)))
    (elif (`/Game/Blueprints/ProdAndTrust/AMJ_Prod.IsFinished` (`self.CurrentProd`))
      (set `self.IsProdTrusting` true)
      (`Actor.K2_DestroyActor` (`self.CurrentProd`))
      (set `self.CurrentProd` null)
      (set `self.Trust` 1.0)
      (set `self.TrustLooseSpeed` (`KismetMathLibrary.RandomFloatInRange` _trustspeedrange_x _trustspeedrange_y)))))

(fn `AttackPerformed`
  (bind _currentprod (`self.CurrentProd`))
  (if (`self.IsProdTrusting`)
    (`self.DecreaseTrust` (`self.TrustLostForAttack`))
    (else
      (`BlackboardComponent.SetValueAsBool` (`AIBlueprintHelperLibrary.GetBlackboard` _currentprod) "WasNaughty" (== (`KismetMathLibrary.VSize` (`Actor.GetVelocity` _currentprod)) 0.0)))))

(fn `DecreaseTrust`
  (params (AmountToDecrease :type "Float (double-precision)"))
  (bind _output_get (set `self.Trust` (- (`self.Trust`) AmountToDecrease)))
  (if (<= _output_get 0.0)
    (set `self.IsProdTrusting` false)
    (`self.SpawnProd`)
    (elif (> _output_get 1.0)
      (set `self.Trust` 1.0))))

(fn `SpawnProd`
  (bind _outactors (`GameplayStatics.GetAllActorsWithTag` "ProdSpawnPosition"))
  (bind _returnvalue (`|SpawnActorFromClass` (`self.ProdClass`) (`Actor.GetTransform` (`|GetArrayItem` _outactors)) "Undefined" "OverrideRootScale"))
  (set `self.CurrentProd` _returnvalue))