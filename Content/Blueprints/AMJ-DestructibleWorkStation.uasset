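; Destructible workstation actor that can be shattered on demand and removes itself after a set lifetime.
; The Destroy function damages the destructible mesh with a strong upward impulse.
; Independently, Tick counts down the lifetime from BeginPlay, then turns off physics on Comp and shrinks it while sinking the destructible.
; The actor is destroyed once the scale reaches zero and the mesh drops below a world height threshold.
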(event `self.ReceiveBeginPlay`
  (set `self.LifeTimeLeft` (`self.TimeOfLife`)))

(event `self.ReceiveTick`
  (params (DeltaSeconds :type "Float (single-precision)"))
  (bind (_returnvalue_x _returnvalue_y _returnvalue_z) (`KismetMathLibrary.BreakVector` (`SceneComponent.K2_GetComponentLocation` (`self.Destructible`))))
  (if (`self.IsFadingOut`)
    (`PrimitiveComponent.SetSimulatePhysics` (`self.Comp`) false)
    (`SceneComponent.K2_AddLocalOffset` (`self.Destructible`) (`KismetMathLibrary.MakeVector` 0.0 0.0 (* DeltaSeconds -50.0)) false false)
    (bind _output_get (set `self.Scale` (- (`self.Scale`) DeltaSeconds)))
    (if (<= _output_get 0.0)
      (bind _output_get_2 (set `self.Scale` 0.0)))
    (`SceneComponent.SetWorldScale3D` (`self.Comp`) (`KismetMathLibrary.MakeVector` _output_get_2 _output_get_2 _output_get_2))
    (if (and (<= (`self.Scale`) 0.0) (< _returnvalue_z -350.0))
      (`self.K2_DestroyActor`))
    (else
      (bind _output_get_3 (set `self.LifeTimeLeft` (- (`self.LifeTimeLeft`) DeltaSeconds)))
      (if (<= _output_get_3 0.0)
        (set `self.IsFadingOut` true)))))

(fn `Destroy`
  (`DestructibleComponent.ApplyDamage` (`self.Destructible`) 1.0 (`self.K2_GetActorLocation`) (0.0 0.0 1.0) 30000.0))

(fn `UserConstructionScript`)