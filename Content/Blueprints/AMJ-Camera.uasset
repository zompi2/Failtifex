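; Shared camera actor that frames two players, following their midpoint in X and Y with an X offset while keeping its own height.
; Each tick, once both player references are valid, it derives a target spring arm length from player separation, with a minimum, and eases toward it using delta time.
; Helper functions assign the players, make this camera player 0's view target, and play a camera shake with a debug print.
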(event `self.ReceiveTick`
  (params (DeltaSeconds :type "Float (single-precision)"))
  (if (`self.ArePlayersValid`)
    (`self.K2_SetActorLocation` (`self.GetDesiredCameraPos`))
    (`self.SetDesiredSpringArmLen`)
    (`self.UpdateArmLen` DeltaSeconds)))

(fn `ArePlayersValid`
  (returns (Out :type Boolean))
  (return (and (`KismetSystemLibrary.IsValid` (`self.Player1_Ref`)) (`KismetSystemLibrary.IsValid` (`self.Player2_Ref`)))))

(fn `ClampCameraHeight`
  (params (In :type "Float (double-precision)"))
  (returns (Out :type "Float (double-precision)"))
  (bind _returnvalue (+ In (`self.SpringArmMod`)))
  (if (< _returnvalue (`self.MinSpringArmHeight`))
    (return (`self.MinSpringArmHeight`))
    (else
      (return _returnvalue))))

(fn `GetDesiredCameraPos`
  (returns (Output :type "Vector Structure"))
  (bind (_returnvalue_x _returnvalue_y _returnvalue_z) (`KismetMathLibrary.BreakVector` (`self.K2_GetActorLocation`)))
  (bind (_returnvalue_x_2 _returnvalue_y_2) (`KismetMathLibrary.BreakVector` (* (+ (`self.K2_GetActorLocation` (`self.Player1_Ref`)) (`self.K2_GetActorLocation` (`self.Player2_Ref`))) 0.5)))
  (return (`KismetMathLibrary.MakeVector` (+ _returnvalue_x_2 (`self.CameraPosXMod`)) _returnvalue_y_2 _returnvalue_z)))

(fn `SetDesiredSpringArmLen`
  (bind _minspringarmheight (`self.MinSpringArmHeight`))
  (bind _returnvalue (+ (* (`KismetMathLibrary.VSize` (- (`self.K2_GetActorLocation` (`self.Player1_Ref`)) (`self.K2_GetActorLocation` (`self.Player2_Ref`)))) (`self.SpringArmMod`)) (`self.SpringArmBaseLen`)))
  (if (< _returnvalue _minspringarmheight)
    (set `self.TargetSpringArmLen` _minspringarmheight)
    (else
      (set `self.TargetSpringArmLen` _returnvalue))))

(fn `SetPlayersToCamera`
  (params (Player1In :type "Actor Object Reference") (Player2In :type "Actor Object Reference"))
  (set `self.Player1_Ref` Player1In)
  (set `self.Player2_Ref` Player2In))

(fn `SetThisCameraToViewport`
  (`PlayerController.SetViewTargetWithBlend` (`GameplayStatics.GetPlayerController` 0) self 0.0 "VTBlend_Linear" 0.0 false))

(fn `Shake`
  (`KismetSystemLibrary.PrintString` "SHAKE")
  (`PlayerController.ClientStartCameraShake` :`self` (`GameplayStatics.GetPlayerController` 0) :`Shake` "/Game/Blueprints/AMJ-CameraShake.AMJ-CameraShake_C" :`Scale` 0.5 :`PlaySpace` "World"))

(fn `UpdateArmLen`
  (params (DeltaTime :type "Float (double-precision)"))
  (bind _springarm (`self.SpringArm`))
  (bind _targetarmlength (`SpringArmComponent.TargetArmLength` _springarm))
  (set `SpringArmComponent.TargetArmLength` (+ (* (- (`self.TargetSpringArmLen`) _targetarmlength) DeltaTime) _targetarmlength) _springarm))

(fn `UserConstructionScript`)